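; BP_MusicHUD drives the on-screen score and result display for a music challenge.
; On BeginPlay it creates score and result widgets for the first player and keeps both disabled.
; Binding to a zone enables the score widget, and score updates are forwarded to it.
; Challenge end notifies both widgets, always passing zero percentage to the result, then disables the result widget after a short delay.
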(event EventBeginPlay
  (bind _returnvalue (Game|GetPlayerController 0))
  (bind _returnvalue_2 (UserInterface|CreateWidget "/Game/Blueprints/WBP_Score.WBP_Score_C" _returnvalue))
  (bind _output_get (Variables|Default|SetScoreWidget _returnvalue_2))
  (UserInterface|Viewport|AddtoViewport _output_get 0)
  (Default|DisableAll (Variables|Default|GetScoreWidget))
  (bind _returnvalue_3 (UserInterface|CreateWidget "/Game/Blueprints/WBP_Result.WBP_Result_C" _returnvalue))
  (bind _output_get_2 (Variables|Default|SetResultWidget _returnvalue_3))
  (UserInterface|Viewport|AddtoViewport _output_get_2 0)
  (Default|DisableAll (Variables|Default|GetResultWidget)))

(event EventOnScoreUpdated
  (params (bSuccess :type Boolean) (SuccessCount :type Integer) (FailCount :type Integer) (Percent :type Float%20%28single-precision%29))
  (Default|ScoreUpdated (Variables|Default|GetScoreWidget) bSuccess SuccessCount FailCount Percent))

(event EventOnChallengeEnded
  (params (bAbandoned :type Boolean) (FinalPercent :type Float%20%28single-precision%29))
  (bind _resultwidget (Variables|Default|GetResultWidget))
  (Development|PrintString "Challenge Ended")
  (Default|ChallengeEnded (Variables|Default|GetScoreWidget))
  (Default|ChallengeEnded _resultwidget bAbandoned 0.0)
  (Utilities|FlowControl|Delay 3.0)
  (Default|DisableAll _resultwidget))

(event EventOnZoneBound
  (params (Zone :type Music%20Zone%20Object%20Reference))
  (Default|EnableAll (Variables|Default|GetScoreWidget)))

(fn ConstructionScript)